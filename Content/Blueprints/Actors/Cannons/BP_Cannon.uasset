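; BP_Cannon is a cannon actor that automatically fires BP_Projectile on a repeating cycle from BeginPlay.
; After a FireRate delay, it spawns a projectile at ProjectileSpawnPoint's world transform, scaled by ProjectileScale.
; CannonFireTimeline then animates barrel recoil along relative Y through its BarrelPull track.
; The timeline's Cannon Fired event loops back to the delay, so no Tick is needed.
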(event EventBeginPlay
  (bind _projectilespawnpoint (Variables|Default|GetProjectileSpawnPoint))
  (Utilities|FlowControl|Delay (Variables|Default|GetFireRate) :!label _label)
  (Game|SpawnActorfromClass "/Game/Blueprints/Actors/Projectiles/BP_Projectile.BP_Projectile_C" (Math|Transform|MakeTransform (Transformation|GetWorldLocation _projectilespawnpoint) (Transformation|GetWorldRotation _projectilespawnpoint) (Math|Conversions|ToVector(Float) (Variables|Default|GetProjectileScale))) "Undefined" 0 0)
  (bind _barrelpull (Timeline|Cannon%20Fire%20Timeline PlayFromStart)
    (:Update
      (Transformation|SetRelativeLocation (Variables|Default|GetCannonBarrel) (Math|Vector|MakeVector 0.0 _barrelpull 0.0) false false))
    (:CannonFired
      (goto _label))))

(event Collision|EventActorBeginOverlap
  (params (OtherActor :type Actor%20Object%20Reference)))

(event EventTick
  (params (DeltaSeconds :type Float%20%28single-precision%29)))

(fn ConstructionScript)